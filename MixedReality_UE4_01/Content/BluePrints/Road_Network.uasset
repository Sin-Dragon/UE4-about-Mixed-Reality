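; Road_Network Blueprint that assigns fixed integer values to cube and cylinder elements, which by its naming represent a road network.
; BeginPlay runs SetCubeValue to number the eight cubes, then SetRoadValue for the cylinders.
; Each value comes from a function named after the constant it returns, ignoring its input.
; Most of SetRoadValue is disconnected, so only Cylinder and Cylinder12 receive values there.
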(event EventBeginPlay
  (CallFunction|SetCubeValue self)
  (CallFunction|SetRoadValue self))

(event Collision|EventActorBeginOverlap
  (params (OtherActor :type Actor%20Object%20Reference)))

(event EventTick
  (params (DeltaSeconds :type Float%20%28single-precision%29)))

(fn ConstructionScript)

(fn 1
  (params (NewParam :type Static%20Mesh%20Component%20Object%20Reference))
  (return 1))

(fn 2
  (params (NewParam :type Static%20Mesh%20Component%20Object%20Reference))
  (return 2))

(fn 3
  (params (NewParam :type Static%20Mesh%20Component%20Object%20Reference))
  (return 3))

(fn 4
  (params (NewParam :type Static%20Mesh%20Component%20Object%20Reference))
  (return 4))

(fn 5
  (params (NewParam :type Static%20Mesh%20Component%20Object%20Reference))
  (return 5))

(fn 6
  (params (NewParam :type Static%20Mesh%20Component%20Object%20Reference))
  (return 6))

(fn 7
  (params (NewParam :type Static%20Mesh%20Component%20Object%20Reference))
  (return 7))

(fn 8
  (params (NewParam :type Static%20Mesh%20Component%20Object%20Reference))
  (return 8))

(fn SetRoadValue
  (bind _self self)
  (bind _newparam1 (CallFunction|4 _self (Variables|Default|GetCylinder)))
  (Variables|Default|SetCylinder_Value _newparam1)
  (bind _newparam1_2 (CallFunction|8 _self (Variables|Default|GetCylinder12)))
  (Variables|Default|SetCylinder12_Value _newparam1_2))

(fn SetCubeValue
  (bind _self self)
  (bind _newparam1 (CallFunction|1 _self (Variables|Default|GetCube)))
  (Variables|Default|SetCube_Value _newparam1)
  (bind _newparam1_2 (CallFunction|2 _self (Variables|Default|GetCube1)))
  (Variables|Default|SetCube1_Value _newparam1_2)
  (bind _newparam1_3 (CallFunction|3 _self (Variables|Default|GetCube3)))
  (Variables|Default|SetCube3_Value _newparam1_3)
  (bind _newparam1_4 (CallFunction|4 _self (Variables|Default|GetCube5)))
  (Variables|Default|SetCube5_Value _newparam1_4)
  (bind _newparam1_5 (CallFunction|5 _self (Variables|Default|GetCube7)))
  (Variables|Default|SetCube7_Value _newparam1_5)
  (bind _newparam1_6 (CallFunction|6 _self (Variables|Default|GetCube6)))
  (Variables|Default|SetCube6_Value _newparam1_6)
  (bind _newparam1_7 (CallFunction|7 _self (Variables|Default|GetCube4)))
  (Variables|Default|SetCube4_Value _newparam1_7)
  (bind _newparam1_8 (CallFunction|8 _self (Variables|Default|GetCube2)))
  (Variables|Default|SetCube2_Value _newparam1_8))

(fn 9
  (params (NewParam :type Static%20Mesh%20Component%20Object%20Reference))
  (return 9))

(fn 10
  (params (NewParam :type Static%20Mesh%20Component%20Object%20Reference))
  (return 10))

(fn 11
  (params (NewParam :type Static%20Mesh%20Component%20Object%20Reference))
  (return 11))

(fn 14
  (params (NewParam :type Static%20Mesh%20Component%20Object%20Reference))
  (return 14))