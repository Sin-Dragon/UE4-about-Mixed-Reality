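; NearMenu is a Blueprint actor that acts as a near menu with two UXT pressable buttons for revealing scene objects.
; On BeginPlay it fetches the pressable button component from each button's child actor and binds a press handler.
; Pressing the first button unhides the slider light actor, and pressing the second unhides the sand table.
; Both handlers only show their targets and never hide them again.
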(event Custom|OnButtonPressed
  (params (Button :type Uxt%20Pressable%20Button%20Component%20Object%20Reference) (Pointer :type Uxt%20Pointer%20Component%20Object%20Reference))
  ;[1 1 1] Button_01(Silder_Light about Sandtable)
  (Rendering|SetActorHiddenInGame (Variables|Default|GetSilder_Light) false))

(event Custom|On%20Button%20Pressed_02
  (params (Button :type Uxt%20Pressable%20Button%20Component%20Object%20Reference) (Pointer :type Uxt%20Pointer%20Component%20Object%20Reference))
  (Rendering|SetActorHiddenInGame (Variables|Default|GetSandTable) false))

(event EventBeginPlay
  (|CallParentFunction)
  ;[1 1 1] Button_01(Silder_Light about Sandtable)
  (EventDispatchers|AssignOnButtonPressed (Actor|GetComponentsByClass (Variables|/Script/Engine.ChildActorComponent|GetChildActor (Variables|Default|GetButton_01)) "/Script/UXTools.UxtPressableButtonComponent") (delegate Custom|OnButtonPressed))
  (EventDispatchers|BindEventtoOnButtonPressed (Actor|GetComponentsByClass (Variables|/Script/Engine.ChildActorComponent|GetChildActor (Variables|Default|GetButton_02)) "/Script/UXTools.UxtPressableButtonComponent") (delegate Custom|On%20Button%20Pressed_02)))

(event Collision|EventActorBeginOverlap
  (params (OtherActor :type Actor%20Object%20Reference))
  (|CallParentFunction OtherActor) ; 此节点被禁用，将不会被调用。\n从引脚连出引线来编译功能。
)

(event EventTick
  (params (DeltaSeconds :type Float%20%28single-precision%29))
  (|CallParentFunction DeltaSeconds) ; 此节点被禁用，将不会被调用。\n从引脚连出引线来编译功能。
)

(fn ConstructionScript
  (|CallParentFunction))